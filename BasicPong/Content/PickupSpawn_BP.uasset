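; PickupSpawn_BP is a spawner actor that keeps adding Pickup_BP actors at random points within a box volume around itself.
; After BeginPlay and a random delay, the SpawnTimer event spawns a pickup, waits another random interval and calls itself, looping indefinitely.
; The BoxExtent variable bounds the spawn area, and the construction script applies it to the Box component so the two match.
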(event `self.ReceiveBeginPlay`
  (`KismetSystemLibrary.Delay` (`KismetMathLibrary.RandomFloatInRange` 10.0 20.0))
  (`self.SpawnTimer`))

(event `SpawnTimer`
  (`|SpawnActorFromClass` "/Game/Pickup_BP.Pickup_BP_C" (`KismetMathLibrary.MakeTransform` (`KismetMathLibrary.RandomPointInBoundingBox` (`self.K2_GetActorLocation`) (`self.BoxExtent`))) "Undefined" "MultiplyWithRoot" null null)
  (`KismetSystemLibrary.Delay` (`KismetMathLibrary.RandomFloatInRange` 10.0 20.0))
  (`self.SpawnTimer`))

(fn `UserConstructionScript`
  (`BoxComponent.SetBoxExtent` (`self.Box`) (`self.BoxExtent`) true))